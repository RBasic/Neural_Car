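; Vehicle Blueprint for a car driven by a neural network component, with manual axis inputs left empty.
; Each active tick feeds five fanned line-trace distances plus normalized forward speed into the network, whose outputs set throttle and steering.
; Fitness decays every tick and grows with speed above a threshold.
; Wall hits or too-low fitness deactivate the network, zeroing the controls while fitness keeps dropping.
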(event OnComponentHit(Mesh)
  (params (HitComponent :type Primitive%20Component%20Object%20Reference) (OtherActor :type Actor%20Object%20Reference) (OtherComp :type Primitive%20Component%20Object%20Reference) (NormalImpulse :type Vector :default "0, 0, 0") (Hit :type Hit%20Result%20Structure%20%28by%20ref%29))
  ;[1 1 1] Desactivate OnCollide
  (Utilities|Casting|CastToBP_WallRound OtherActor
    (:then
      _)
    (:CastFailed
      (Utilities|Casting|CastToBP_WallStraight OtherActor)))
  (Variables|/Game/Blueprints/Neural/AC_NeuralNetwork.AC_NeuralNetwork_C|SetActive? (Variables|Default|GetAC_NeuralNetwork) false))

(event Custom|MoveForwardNN
  (params (Throttle :type Float%20%28single-precision%29))
  ;[1 1 1] Movement control
  (Class|WheeledVehicleMovementComponent|SetThrottleInput (Variables|Default|GetVehicleMovement) Throttle))

(event Custom|MoveRightNN
  (params (Steering :type Float%20%28single-precision%29))
  ;[1 1 1] Movement control
  (Class|WheeledVehicleMovementComponent|SetSteeringInput (Variables|Default|GetVehicleMovement) Steering))

(event EventTick
  (params (DeltaSeconds :type Float%20%28single-precision%29))
  (bind _vehiclemovement (Variables|Default|GetVehicleMovement))
  (bind _scene (Variables|Default|GetScene))
  (bind _ac_neuralnetwork (Variables|Default|GetAC_NeuralNetwork))
  (bind _ac_neuralnetwork_2 (Variables|Default|GetAC_NeuralNetwork))
  (bind _returnvalue (Class|WheeledVehicleMovementComponent|GetForwardSpeed _vehiclemovement))
  (bind _returnvalue_2 (Transformation|GetWorldLocation _scene))
  ;[1 1 1] BIG EVENT TICK TO CHANGE
  (Default|AddFitness _ac_neuralnetwork -0.2)
  (if (Variables|/Game/Blueprints/Neural/AC_NeuralNetwork.AC_NeuralNetwork_C|GetActive? _ac_neuralnetwork)
    (Utilities|FlowControl|Sequence
      (:then_0
        (if (<= (Default|GetFitness _ac_neuralnetwork_2) -15.0)
          (Variables|/Game/Blueprints/Neural/AC_NeuralNetwork.AC_NeuralNetwork_C|SetActive? _ac_neuralnetwork_2 false)))
      (:then_1
        (if (>= _returnvalue 2e+02)
          (Default|AddFitness (Variables|Default|GetAC_NeuralNetwork) (* 0.001 (Math|Float|Absolute(Float) _returnvalue)))))
      (:then_2
        (for _index (range 0 4)
          (bind _outhit (Collision|LineTraceForObjects _returnvalue_2 (+ _returnvalue_2 (* (Math|Vector|RotateVector (Math|Vector|GetForwardVector (Variables|Default|GetScene)) (Math|Rotator|MakeRotator 0.0 0.0 (Utilities|Select :Index _index :Option%200 -6e+01 :Option%201 -3e+01 :Option%202 0.0 :Option%203 3e+01 :Option%204 6e+01))) (Variables|Default|GetmaxDistRaycast))) (Utilities|Array|MakeArray "ObjectTypeQuery2" "ObjectTypeQuery1") false 0 "ForOneFrame"))
          (Utilities|Array|SetArrayElem (Variables|Default|GetInputsArray) _index (/ (.distance _outhit) (Variables|Default|GetmaxDistRaycast)))))
      (:then_3
        (Utilities|Array|SetArrayElem (Variables|Default|GetInputsArray) 5 (/ (Class|WheeledVehicleMovementComponent|GetForwardSpeed (Variables|Default|GetVehicleMovement)) (Variables|Default|GetmaxSpeed)))
        (bind _outputs (Default|FeedForward (Variables|Default|GetAC_NeuralNetwork) (Variables|Default|GetInputsArray)))
        (CallFunction|MoveForwardNN (Utilities|Array|Get(acopy) _outputs))
        (CallFunction|MoveRightNN (Utilities|Array|Get(acopy) _outputs 1))))
    (else
      (CallFunction|MoveForwardNN 0.0)
      (CallFunction|MoveRightNN 0.0)
      (Default|AddFitness (Variables|Default|GetAC_NeuralNetwork) -0.2))))

(event Input|AxisEvents|InputAxisMoveForward
  (params (AxisValue :type Float%20%28single-precision%29))
  ;[1 1 1] Movement control
)

(event Input|AxisEvents|InputAxisMoveRight
  (params (AxisValue :type Float%20%28single-precision%29))
  ;[1 1 1] Movement control
)

(fn ConstructionScript)