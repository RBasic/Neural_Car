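; Neural network component with a fitness score, weight copying and mutation, as used for evolutionary training without backpropagation.
; InitializeNetwork builds neuron layers from a size array and randomizes the nested-struct weight arrays.
; FeedForward computes bias-free weighted sums layer by layer through a switchable sigmoid or tanh activation and returns the last layer.
; Mutate re-rolls each weight at a given probability, and print helpers dump neurons and weights.
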(fn InitializeNetwork
  (params (Layers :type Array%20of%20Integers))
  (Variables|Config|SetLayers Layers)
  (Variables|Config|SetFitness 0.0)
  (Initialization|InitializeNeurons)
  (Initialization|InitializeWeights)
  (Variables|Config|SetActive? true))

(fn InitializeNeurons
  (bind _neurons (Variables|Config|GetNeurons))
  (for (_array_element _array_index) (Variables|Config|GetLayers)
    (Utilities|Array|Add _neurons (Utilities|Struct|MakeStruct_2DArray 0))
    (Utilities|Array|Resize (.struct1d (Utilities|Array|Get(acopy) _neurons _array_index)) _array_element)))

(fn InitializeWeights
  (for _index (range 1 (Utilities|Array|LastIndex (Variables|Config|GetLayers)))
    (Utilities|Array|Clear (LocalVariables|GetlayerWeightsList))
    (LocalVariables|SetNeuronsInPreviousLayer (Utilities|Array|Get(acopy) (Variables|Config|GetLayers) (- _index 1)))
    (for _array_element (.struct1d (Utilities|Array|Get(acopy) (Variables|Config|GetNeurons) _index))
      (Utilities|Array|Clear (LocalVariables|GetNeuronsWeights))
      (Utilities|Array|Resize (LocalVariables|GetNeuronsWeights) (LocalVariables|GetNeuronsInPreviousLayer))
      (for (_ _array_index) (LocalVariables|GetNeuronsWeights)
        (Utilities|Array|SetArrayElem (LocalVariables|GetNeuronsWeights) _array_index (Math|Random|RandomFloatinRange -1.0 1.0)))
      (Utilities|Array|Add (LocalVariables|GetlayerWeightsList) (Utilities|Struct|MakeStruct_2DArray (LocalVariables|GetNeuronsWeights))))
    (Utilities|Array|Add (LocalVariables|GetweightList) (Utilities|Struct|MakeStruct_3DArray (LocalVariables|GetlayerWeightsList))))
  (Variables|Config|SetWeights (LocalVariables|GetweightList)))

(fn PrintNeurons
  (params (Duration :type Float%20%28single-precision%29))
  (for (_array_element _array_index) (Variables|Config|GetNeurons)
    (for (_array_element_2 _array_index_2) (.struct1d _array_element)
      (Development|PrintString (Utilities|String|ToString(Text) (Utilities|Text|FormatText "tab[{i}][{j}]={element}" _array_index _array_index_2 _array_element_2)) true true "(R=0.000000,G=0.660000,B=1.000000,A=1.000000)" Duration))))

(fn PrintWeights
  (params (Duration :type Float%20%28single-precision%29))
  (for (_array_element _array_index) (Variables|Config|GetWeights)
    (for (_array_element_2 _array_index_2) (.struct2d _array_element)
      (for (_array_element_3 _array_index_3) (.struct1d _array_element_2)
        (Development|PrintString (Utilities|String|ToString(Text) (Utilities|Text|FormatText "tab[{i}][{j}][{k}]={element}" _array_index _array_index_2 _array_index_3 _array_element_3)) true true "(R=0.000000,G=0.660000,B=1.000000,A=1.000000)" Duration)))))

(fn CopyWeights
  (params (CopyWeights :type Array%20of%20Struct%203D%20Array%20Structures))
  (for (_array_element _array_index) CopyWeights
    (for (_array_element_2 _array_index_2) (.struct2d _array_element)
      (for (_array_element_3 _array_index_3) (.struct1d _array_element_2)
        (Utilities|Array|SetArrayElem (.struct1d (Utilities|Array|Get(acopy) (.struct2d (Utilities|Array|Get(acopy) (Variables|Config|GetWeights) _array_index)) _array_index_2)) _array_index_3 _array_element_3)))))

(fn AddFitness
  (params (fit :type Float%20%28single-precision%29))
  (Variables|Config|SetFitness (+ fit (Variables|Config|GetFitness))))

(fn FeedForward
  (params (inputs :type Array%20of%20Floats%20%28single-precision%29))
  (bind _neurons (Variables|Config|GetNeurons))
  (|SetBy-RefVar (.struct1d (Utilities|Array|Get(acopy) (Variables|Config|GetNeurons))) inputs)
  (for _index (range 1 (Utilities|Array|LastIndex (Variables|Config|GetLayers)))
    (for _index_2 (range 0 (Utilities|Array|LastIndex (.struct1d (Utilities|Array|Get(acopy) (Variables|Config|GetNeurons) _index))))
      (LocalVariables|Setval 0.0)
      (for _index_3 (range 0 (Utilities|Array|LastIndex (.struct1d (Utilities|Array|Get(acopy) (Variables|Config|GetNeurons) (- _index 1)))))
        (LocalVariables|Setval (+ (LocalVariables|Getval) (* (Utilities|Array|Get(acopy) (.struct1d (Utilities|Array|Get(acopy) (.struct2d (Utilities|Array|Get(acopy) (Variables|Config|GetWeights) (- _index 1))) _index_2)) _index_3) (Utilities|Array|Get(acopy) (.struct1d (Utilities|Array|Get(acopy) (Variables|Config|GetNeurons) (- _index 1))) _index_3)))))
      (Utilities|Array|SetArrayElem (.struct1d (Utilities|Array|Get(acopy) (Variables|Config|GetNeurons) _index)) _index_2 (Math|Float|SelectFloat (Tools|Sigmoid (LocalVariables|Getval)) (Tools|HyperbolicTangent (LocalVariables|Getval)) (Variables|Default|GetSigmoid?)))))
  (return (.struct1d (Utilities|Array|Get(acopy) _neurons (Utilities|Array|LastIndex _neurons)))))

(fn HyperbolicTangent
  (params (Val :type Float%20%28single-precision%29))
  (return (|((1-(e(((0-2)*z))))/(1+(e(((0-2)*z))))) Val)))

(fn Sigmoid
  (params (A :type Float%20%28single-precision%29))
  (return (|(1/(1+(e((0-x))))) A)))

(fn Mutate
  (params (Condition :type Float%20%28single-precision%29))
  (for (_array_element _array_index) (Variables|Config|GetWeights)
    (for (_array_element_2 _array_index_2) (.struct2d _array_element)
      (for (_array_element_3 _array_index_3) (.struct1d _array_element_2)
        (Utilities|Array|SetArrayElem (.struct1d (Utilities|Array|Get(acopy) (.struct2d (Utilities|Array|Get(acopy) (Variables|Config|GetWeights) _array_index)) _array_index_2)) _array_index_3 (Math|Float|SelectFloat (Math|Random|RandomFloatinRange -1.0 1.0) _array_element_3 (<= (Math|Random|RandomFloat) Condition)))))))

(fn SetFitness
  (params (Fitness :type Float%20%28single-precision%29))
  (Variables|Config|SetFitness Fitness))

(fn GetFitness
  (return (Variables|Config|GetFitness)))

(fn GetOutputs
  (bind _neurons (Variables|Config|GetNeurons))
  (return (.struct1d (Utilities|Array|Get(acopy) _neurons (Utilities|Array|LastIndex _neurons)))))