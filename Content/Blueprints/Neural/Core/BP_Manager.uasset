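; Manager actor that runs a neuroevolution simulation, spawning a population of actors with AC_NeuralNetwork components.
; When none are active or a restart is forced, it selects the fittest fraction, copies and mutates their weights, then respawns everyone at its transform.
; Keys save the best network to the "Weights" slot, which seeds the population on BeginPlay, or reset, restart and change time dilation.
; On-screen debug shows outputs and fitness.
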(event Custom|InitActors
  ;[1 1 1] InitActors
  (for _index (range 1 (Variables|Default|GetnbActors))
    (bind _returnvalue (Game|SpawnActorfromClass (Variables|Default|GetActorClass) (Transformation|GetActorTransform) "AlwaysSpawn" 0 0))
    (Utilities|Array|Add (Variables|Default|GetNeurals) (Actor|GetComponentbyClass _returnvalue "/Game/Blueprints/Neural/Core/AC_NeuralNetwork.AC_NeuralNetwork_C"))
    (Variables|/Game/Blueprints/Neural/Core/AC_NeuralNetwork.AC_NeuralNetwork_C|SetSigmoid? (Actor|GetComponentbyClass _returnvalue "/Game/Blueprints/Neural/Core/AC_NeuralNetwork.AC_NeuralNetwork_C") (Variables|Default|GetSigmoid?))
    (Default|InitializeNetwork (Actor|GetComponentbyClass _returnvalue "/Game/Blueprints/Neural/Core/AC_NeuralNetwork.AC_NeuralNetwork_C") (Variables|Default|GetLayer))))

(event Custom|Respawn
  ;[1 1 1] Respawn at Manager transform
  (for _array_element (Variables|Default|GetNeurals)
    (Transformation|SetActorTransform (Components|GetOwner _array_element) (Transformation|GetActorTransform) false true)
    (Default|SetFitness _array_element 0.0)
    (Variables|/Game/Blueprints/Neural/Core/AC_NeuralNetwork.AC_NeuralNetwork_C|SetActive? _array_element true)))

(event Custom|InitSave
  ;[1 1 1] Save Weights in save slot
  (bind _returnvalue (SaveGame|DoesSaveGameExist "Weights"))
  (if _returnvalue
    (bind _returnvalue_2 (SaveGame|LoadGamefromSlot "Weights"))
    (bind _asbp_save_weights (Utilities|Casting|CastToBP_SaveWeights _returnvalue_2))
    (bind _output_get (Variables|Default|SetSave _asbp_save_weights))
    (for _array_element (Variables|Default|GetNeurals)
      (Default|CopyWeights _array_element (Variables|/Game/Blueprints/Neural/Core/BP_SaveWeights.BP_SaveWeights_C|GetWeights _output_get)))
    (CallFunction|NextGen (Variables|Default|GetMutationValue) (Variables|Default|GetBestPercent))
    (else
      (bind _returnvalue_3 (SaveGame|CreateSaveGameObject "/Game/Blueprints/Neural/Core/BP_SaveWeights.BP_SaveWeights_C"))
      (Variables|Default|SetSave _returnvalue_3))))

(event Custom|BestSaved
  (params (Weights :type Array%20of%20Struct%203D%20Array%20Structures))
  (bind _save (Variables|Default|GetSave))
  ;[1 1 1] Save actual best neural
  (Variables|/Game/Blueprints/Neural/Core/BP_SaveWeights.BP_SaveWeights_C|SetWeights _save Weights)
  (bind _returnvalue (SaveGame|SaveGametoSlot _save "Weights"))
  (Development|PrintString (Utilities|String|SelectString "Saved" "Not Saved" _returnvalue) true true "(R=1.000000,G=0.041493,B=0.000000,A=1.000000)" 5e+01))

(event EventTick
  (params (DeltaSeconds :type Float%20%28single-precision%29))
  ;[1 1 1] Event tick
  (Utilities|FlowControl|Sequence
    (:then_0
      (CallFunction|Debug))
    (:then_1
      (bind _noactive_ (CallFunction|NoActorActive? (Variables|Default|GetNeurals)))
      (if (or _noactive_ (Variables|Default|GetBigRedButton?))
        (Variables|Default|SetBigRedButton? false)
        (CallFunction|NextGen (Variables|Default|GetMutationValue) (Variables|Default|GetBestPercent))))))

(event EventBeginPlay
  ;[1 1 1] BeginPlay
  (bind _canlaunch_ (CallFunction|CheckInputs))
  (if _canlaunch_
    (CallFunction|InitActors)
    (CallFunction|InitSave)))

(event Input|KeyboardEvents|Add
  (params (Key :type Key%20Structure :default "None"))
  ;[1 1 1] Time Dilation
  (:Pressed
    (Utilities|Time|SetGlobalTimeDilation (Math|Float|Clamp(Float) (+ (Class|GameplayStatics|GetGlobalTimeDilation) 1.0) 1.0 2e+01))))

(event Input|KeyboardEvents|Subtract
  (params (Key :type Key%20Structure :default "None"))
  ;[1 1 1] Time Dilation
  (:Pressed
    (Utilities|Time|SetGlobalTimeDilation (Math|Float|Clamp(Float) (- (Class|GameplayStatics|GetGlobalTimeDilation) 1.0) 1.0 2e+01))))

(event Input|KeyboardEvents|SpaceBar
  (params (Key :type Key%20Structure :default "None"))
  ;[1 1 1] RestartSimulation
  (:Pressed
    (Variables|Default|SetBigRedButton? true)))

(event Input|KeyboardEvents|E
  (params (Key :type Key%20Structure :default "None"))
  ;[1 1 1] Save actual best neural
  (:Pressed
    (bind _bests (CallFunction|GetBestActors (Variables|Default|GetNeurals) (Variables|Default|GetBestPercent)))
    (CallFunction|BestSaved (Variables|/Game/Blueprints/Neural/Core/AC_NeuralNetwork.AC_NeuralNetwork_C|GetWeights (Utilities|Array|Get(acopy) _bests)))))

(event Input|KeyboardEvents|R
  (params (Key :type Key%20Structure :default "None"))
  ;[1 1 1] Reset ALL simulation
  (:Pressed
    (CallFunction|NextGen 1.0 (Variables|Default|GetBestPercent))
    (SaveGame|DeleteGameinSlot "Weights")
    (CallFunction|InitSave)))

(fn ConstructionScript)

(fn NoActorActive?
  (params (Array :type Array%20of%20AC%20Neural%20Network%20Object%20References))
  (for _array_element Array
    (if (Variables|/Game/Blueprints/Neural/Core/AC_NeuralNetwork.AC_NeuralNetwork_C|GetActive? _array_element)
      (return false)))
  (return true))

(fn GetBestActors
  (params (InputNeurals :type Array%20of%20AC%20Neural%20Network%20Object%20References) (BestPercent :type Float%20%28single-precision%29))
  (LocalVariables|SetCopyNeurals InputNeurals)
  (for _index (range 1 (Math|Float|Ceil (* (Math|Conversions|ToFloat(Integer) (Utilities|Array|Length InputNeurals)) BestPercent)))
    (while (Utilities|Array|ContainsItem (LocalVariables|GetCheckedIndex) (LocalVariables|GetBestIndex))
      (Math|Integer|IncrementInt (LocalVariables|GetBestIndex)))
    (LocalVariables|SetTempFitness (Default|GetFitness (Utilities|Array|Get(acopy) (LocalVariables|GetCopyNeurals) (LocalVariables|GetBestIndex))))
    (for (_array_element _array_index) (LocalVariables|GetCopyNeurals)
      (if (and (> (Default|GetFitness _array_element) (LocalVariables|GetTempFitness)) (not (Utilities|Array|ContainsItem (LocalVariables|GetCheckedIndex) _array_index)))
        (LocalVariables|SetTempFitness (Default|GetFitness _array_element))
        (LocalVariables|SetBestIndex _array_index)))
    (Utilities|Array|Add (LocalVariables|GetBestNeurals) (Utilities|Array|Get(acopy) (LocalVariables|GetCopyNeurals) (LocalVariables|GetBestIndex)))
    (Utilities|Array|Add (LocalVariables|GetCheckedIndex) (LocalVariables|GetBestIndex))
    (LocalVariables|SetBestIndex 0))
  (return (LocalVariables|GetBestNeurals)))

(fn CopyNextGeneration
  (params (Neurals :type Array%20of%20AC%20Neural%20Network%20Object%20References) (Bests :type Array%20of%20AC%20Neural%20Network%20Object%20References) (Mutation :type Float%20%28single-precision%29))
  (for _index (range 1 (Math|Float|Truncate (/ 1.0 (Variables|Default|GetBestPercent))))
    (for _index_2 (range 0 (Utilities|Array|LastIndex Bests))
      (Utilities|Array|Add (LocalVariables|GetTempNeural) (Utilities|Array|Get(acopy) Bests (- _index 1)))
      (Default|Mutate (Utilities|Array|Get(acopy) Bests (- _index 1)) 0.5)))
  (for (_array_element _array_index) (Variables|Default|GetNeurals)
    (Default|CopyWeights _array_element (Variables|/Game/Blueprints/Neural/Core/AC_NeuralNetwork.AC_NeuralNetwork_C|GetWeights (Utilities|Array|Get(acopy) (LocalVariables|GetTempNeural) _array_index)))))

(fn Debug
  (for (_array_element _array_index) (Variables|Default|GetNeurals)
    (LocalVariables|SetoutputString (Utilities|String|Append "Actor[" (Utilities|String|ToString(Integer) _array_index) "] = {"))
    (for (_array_element_2 _array_index_2) (Default|GetOutputs _array_element)
      (LocalVariables|SetoutputString (Utilities|String|Append (LocalVariables|GetoutputString) (Utilities|String|ToString(Float) _array_element_2) (Utilities|String|SelectString "}" ", " (>= _array_index_2 (Utilities|Array|LastIndex (Default|GetOutputs _array_element)))))))
    (Development|PrintString (Utilities|String|Append (LocalVariables|GetoutputString) " Fitness = " (Utilities|String|ToString(Float) (Default|GetFitness _array_element))) true true (Math|Color|SelectColor "(R=0.071067,G=0.432292,B=0.000000,A=1.000000)" "(R=0.682292,G=0.024300,B=0.000000,A=1.000000)" (Variables|/Game/Blueprints/Neural/Core/AC_NeuralNetwork.AC_NeuralNetwork_C|GetActive? _array_element)) 0.001)
    (LocalVariables|SetoutputString ""))
  (Development|PrintString (Utilities|String|Append "speed x" (Utilities|String|ToString(Float) (Class|GameplayStatics|GetGlobalTimeDilation))) true true "(R=0.000000,G=0.660000,B=1.000000,A=1.000000)" 0.001)
  (bind _returnvalue (SaveGame|DoesSaveGameExist "Weights"))
  (Development|PrintString (Utilities|String|SelectString "SaveGame Existed" "No SaveGame" _returnvalue) true true "(R=0.000000,G=0.660000,B=1.000000,A=1.000000)" 0.001))

(fn CheckInputs
  (bind _actorclass (Variables|Default|GetActorClass))
  (bind _layer (Variables|Default|GetLayer))
  (bind _nbactors (Variables|Default|GetnbActors))
  (bind _bestpercent (Variables|Default|GetBestPercent))
  (bind _returnvalue (Utilities|Array|Length _layer))
  (bind _returnvalue_2 (Utilities|IsValidClass _actorclass))
  (bind _returnvalue_3 (>= _bestpercent 0.01))
  (bind _returnvalue_4 (> _nbactors 0))
  (bind _returnvalue_5 (> _returnvalue 2))
  (Development|PrintString (Utilities|String|ToString(Text) (Utilities|Text|FormatText "Check class = {class} 
Check Layers = {layers} 
check nbBests = {nbBests} 
check nbActors = {nbActors}" _returnvalue_2 _returnvalue_5 _returnvalue_3 _returnvalue_4)))
  (return (Math|Boolean|ANDBoolean _returnvalue_2 _returnvalue_5 _returnvalue_3 _returnvalue_4)))

(fn NextGen
  (params (Mutation :type Float%20%28single-precision%29) (nbBests :type Float%20%28single-precision%29))
  (bind _bests (CallFunction|GetBestActors (Variables|Default|GetNeurals) nbBests))
  (CallFunction|CopyNextGeneration (Variables|Default|GetNeurals) _bests Mutation)
  (CallFunction|Respawn))