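; Manager actor that trains neural-network-driven vehicles through generational evolution.
; It spawns a population of vehicles, each with an initialized network, and waits on Tick until none is active.
; It then picks the top quarter by fitness, copies their weights across four groups with increasing mutation, and respawns all cars at its transform.
; Add and Subtract keys adjust global time dilation to control simulation speed.
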(event Custom|InitCars
  ;[1 1 1] Initialize
  (if (<= (Utilities|Array|Length (Variables|Default|GetCars)) 0)
    (for _index (range 1 (Variables|Default|GetnbActors))
      (bind _returnvalue (Game|SpawnActorfromClass "/Game/VehicleAdvBP/Blueprints/VehicleBlueprint.VehicleBlueprint_C" (Transformation|GetActorTransform) "AlwaysSpawn" 0 0))
      (Utilities|Array|Add (Variables|Default|GetCars) _returnvalue)
      (Default|InitializeNetwork (Variables|/Game/VehicleAdvBP/Blueprints/VehicleBlueprint.VehicleBlueprint_C|GetAC_NeuralNetwork _returnvalue) (Variables|Default|GetLayer))
      (Variables|/Game/VehicleAdvBP/Blueprints/VehicleBlueprint.VehicleBlueprint_C|SetActive _returnvalue true))))

(event Custom|Respawn
  ;[1 1 1] Respawn at Manager transform
  (for _array_element (Variables|Default|GetCars)
    (Transformation|SetActorTransform _array_element (Transformation|GetActorTransform) false true)
    (Default|SetFitness (Variables|/Game/VehicleAdvBP/Blueprints/VehicleBlueprint.VehicleBlueprint_C|GetAC_NeuralNetwork _array_element) 0.0)
    (Variables|/Game/VehicleAdvBP/Blueprints/VehicleBlueprint.VehicleBlueprint_C|SetActive _array_element true)))

(event EventBeginPlay
  ;[1 1 1] InitActorsOnBegin
  (CallFunction|InitCars))

(event EventTick
  (params (DeltaSeconds :type Float%20%28single-precision%29))
  ;[1 1 1] Check if no actors is still active
  (bind _oneactive_ (CallFunction|NoActorActive? (Variables|Default|GetCars)))
  (if _oneactive_
    (bind _best (CallFunction|GetBestActors (Variables|Default|GetCars)))
    (Variables|Default|SetBest _best)
    (CallFunction|NextGenCopy)
    (CallFunction|Respawn)))

(event Input|KeyboardEvents|Add
  (params (Key :type Key%20Structure :default "None"))
  (:Pressed
    (Utilities|Time|SetGlobalTimeDilation (+ (Class|GameplayStatics|GetGlobalTimeDilation) 1.0))
    (Development|PrintString (Utilities|String|Append "speed x" (Utilities|String|ToString(Float) (Class|GameplayStatics|GetGlobalTimeDilation))) true true "(R=0.000000,G=0.660000,B=1.000000,A=1.000000)" 1.0)))

(event Input|KeyboardEvents|Subtract
  (params (Key :type Key%20Structure :default "None"))
  (:Pressed
    (Utilities|Time|SetGlobalTimeDilation (- (Class|GameplayStatics|GetGlobalTimeDilation) 1.0))))

(fn ConstructionScript)

(fn GetBestActors
  (params (Array :type Array%20of%20Vehicle%20Blueprint%20Object%20References))
  (LocalVariables|SetCopyActors Array)
  (for _index (range 1 (/ (Variables|Default|GetnbActors) 4))
    (LocalVariables|SetTempFitness (Default|GetFitness (Variables|/Game/VehicleAdvBP/Blueprints/VehicleBlueprint.VehicleBlueprint_C|GetAC_NeuralNetwork (Utilities|Array|Get(acopy) (LocalVariables|GetCopyActors)))))
    (for (_array_element _array_index) (LocalVariables|GetCopyActors)
      (if (> (Default|GetFitness (Variables|/Game/VehicleAdvBP/Blueprints/VehicleBlueprint.VehicleBlueprint_C|GetAC_NeuralNetwork _array_element)) (LocalVariables|GetTempFitness))
        (LocalVariables|SetTempFitness (Default|GetFitness (Variables|/Game/VehicleAdvBP/Blueprints/VehicleBlueprint.VehicleBlueprint_C|GetAC_NeuralNetwork _array_element)))
        (LocalVariables|SetBestIndex _array_index)))
    (Utilities|Array|Add (LocalVariables|GetBestActors) (Utilities|Array|Get(acopy) (LocalVariables|GetCopyActors) (LocalVariables|GetBestIndex)))
    (Utilities|Array|RemoveIndex (LocalVariables|GetCopyActors) (LocalVariables|GetBestIndex)))
  (return (LocalVariables|GetBestActors)))

(fn NoActorActive?
  (params (Array :type Array%20of%20Vehicle%20Blueprint%20Object%20References))
  (for _array_element Array
    (if (Variables|/Game/VehicleAdvBP/Blueprints/VehicleBlueprint.VehicleBlueprint_C|GetActive _array_element)
      (return false)))
  (return true))

(fn NextGenCopy
  (LocalVariables|SetCarsIndex 0)
  (for _index (range 0 3)
    (for (_array_element _array_index) (Variables|Default|GetBest)
      (Default|CopyOtherWeights (Variables|/Game/VehicleAdvBP/Blueprints/VehicleBlueprint.VehicleBlueprint_C|GetAC_NeuralNetwork (Utilities|Array|Get(acopy) (Variables|Default|GetCars) (LocalVariables|GetCarsIndex))) (Variables|/Game/Blueprints/Neural/AC_NeuralNetwork.AC_NeuralNetwork_C|GetWeights (Variables|/Game/VehicleAdvBP/Blueprints/VehicleBlueprint.VehicleBlueprint_C|GetAC_NeuralNetwork _array_element)))
      (Default|Mutate (Variables|/Game/VehicleAdvBP/Blueprints/VehicleBlueprint.VehicleBlueprint_C|GetAC_NeuralNetwork (Utilities|Array|Get(acopy) (Variables|Default|GetCars) (LocalVariables|GetCarsIndex))) (Utilities|Select :Index _index :Option%200 0.0 :Option%201 0.05 :Option%202 0.075 :Option%203 0.09))
      (Development|PrintString (Utilities|String|Append "Copy best " (Utilities|String|ToString(Integer) _array_index) " into " (Utilities|String|ToString(Integer) (LocalVariables|GetCarsIndex)) " with mutate " (Utilities|String|ToString(Integer) _index)))
      (Math|Integer|IncrementInt (LocalVariables|GetCarsIndex)))))