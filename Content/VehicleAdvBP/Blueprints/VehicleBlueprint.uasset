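; Vehicle pawn driven by a neural network component instead of player input; the MoveForward and MoveRight axis events are empty.
; Each tick while active, five forward-fanned line traces measure distances to WorldDynamic objects and join the vehicle's speed as network inputs.
; The network's two outputs set throttle and steering on the vehicle movement component.
; Hitting a round or straight wall Blueprint clears the Active flag once, halting network control.
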(event OnComponentHit(Mesh)
  (params (HitComponent :type Primitive%20Component%20Object%20Reference) (OtherActor :type Actor%20Object%20Reference) (OtherComp :type Primitive%20Component%20Object%20Reference) (NormalImpulse :type Vector :default "0, 0, 0") (Hit :type Hit%20Result%20Structure%20%28by%20ref%29))
  (Utilities|Casting|CastToBP_WallRound OtherActor
    (:then
      _)
    (:CastFailed
      (Utilities|Casting|CastToBP_WallStraight OtherActor)))
  (Utilities|FlowControl|DoOnce false
    (:Completed
      (Variables|Default|SetActive false))))

(event Custom|MoveForwardNN
  (params (Throttle :type Float%20%28single-precision%29))
  ;[1 1 1] Movement control
  (Class|WheeledVehicleMovementComponent|SetThrottleInput (Variables|Default|GetVehicleMovement) Throttle))

(event Custom|MoveRightNN
  (params (Steering :type Float%20%28single-precision%29))
  ;[1 1 1] Movement control
  (Class|WheeledVehicleMovementComponent|SetSteeringInput (Variables|Default|GetVehicleMovement) Steering))

(event EventBeginPlay
  (Default|InitializeNetwork (Variables|Default|GetAC_NeuralNetwork)))

(event EventTick
  (params (DeltaSeconds :type Float%20%28single-precision%29))
  (bind _scene (Variables|Default|GetScene))
  (bind _returnvalue (Transformation|GetWorldLocation _scene))
  (if (Variables|Default|GetActive)
    (for _index (range 0 4)
      (bind _outhit (Collision|LineTraceForObjects _returnvalue (+ _returnvalue (* (Math|Vector|RotateVector (Math|Vector|GetForwardVector _scene) (Math|Rotator|MakeRotator 0.0 0.0 (Utilities|Select :Index _index :Option%200 -6e+01 :Option%201 -3e+01 :Option%202 0.0 :Option%203 3e+01 :Option%204 6e+01))) 1e+04)) (Utilities|Array|MakeArray "ObjectTypeQuery2") false 0 "ForOneFrame"))
      (Utilities|Array|SetArrayElem (Variables|Default|GetInputsArray) _index (.distance _outhit)))
    (Utilities|Array|SetArrayElem (Variables|Default|GetInputsArray) 5 (Math|Vector|VectorLength (Transformation|GetVelocity)))
    (bind _outputs (Default|FeedForward (Variables|Default|GetAC_NeuralNetwork) (Variables|Default|GetInputsArray)))
    (CallFunction|MoveForwardNN (Utilities|Array|Get(acopy) _outputs))
    (CallFunction|MoveRightNN (Utilities|Array|Get(acopy) _outputs 1))
    (Default|PrintOutput (Variables|Default|GetAC_NeuralNetwork))))

(event Input|AxisEvents|InputAxisMoveForward
  (params (AxisValue :type Float%20%28single-precision%29))
  ;[1 1 1] Movement control
)

(event Input|AxisEvents|InputAxisMoveRight
  (params (AxisValue :type Float%20%28single-precision%29))
  ;[1 1 1] Movement control
)

(fn ConstructionScript)